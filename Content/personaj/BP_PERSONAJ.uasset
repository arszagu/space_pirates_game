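; Player character Blueprint that handles movement, two switchable cameras, interaction, pistol equipping and attacking.
; Axis input drives movement and look, while a Sequence overrides walk speed for backward, sprint and strafe states.
; A short trace from Extracamera messages BP_UI actors and sets HasPistol, unlocking a FlipFlop that moves the pistol between two mesh sockets.
; Camera toggling also switches controller yaw rotation; attack plays a montage once the pistol is equipped.
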(event `InputAction|action`
  (params (Key :type "Key Structure"))
  (bind _extracamera (`self.extracamera`))
  (bind _returnvalue (`SceneComponent.K2_GetComponentLocation` _extracamera))
  ;[1 1 1] лучи
  (:`Pressed`
    (bind (_outhit _returnvalue_2) (`KismetSystemLibrary.LineTraceSingle` :`Start` _returnvalue :`End` (+ _returnvalue (* (`SceneComponent.GetForwardVector` _extracamera) 200.0)) :`TraceChannel` "TraceTypeQuery1" :`DrawDebugType` "ForDuration"))
    (if _returnvalue_2
      (bind (_bblockinghit _binitialoverlap _time _distance _location _impactpoint _normal _impactnormal _physmat _hitactor) (`GameplayStatics.BreakHitResult` _outhit))
      (if (`KismetSystemLibrary.DoesImplementInterface` _hitactor "/Game/personaj/BP_UI.BP_UI_C")
        (message `/Game/personaj/BP_UI.interact` _hitactor)
        (set `self.has pistol?` true)))))

(event `InputAction|sprint`
  (params (Key :type "Key Structure"))
  ;[1 1 1] бег
  (:`Pressed`
    (if (== (stale `InputAxis|forward` AxisValue) 1.0)
      (set `self.is sprinting?` true)
      (else
        (set `self.is sprinting?` false))))
  (:`Released`
    (set `self.is sprinting?` false)))

(event `InputAxis|forward`
  (params (AxisValue :type "Float (single-precision)"))
  (bind _charactermovement (`self.CharacterMovement`))
  ;[1 1 1] передвежение
  (`self.AddMovementInput` (`SceneComponent.GetForwardVector` (`self.CapsuleComponent`)) AxisValue)
  (`|ExecutionSequence`
    (:`then_0`
      ;[1 1 1] вперед
      (set `CharacterMovementComponent.MaxWalkSpeed` 300.0 _charactermovement))
    (:`then_1`
      ;[1 1 1] смена камеры
      (if (== AxisValue -1.0)
        (set `CharacterMovementComponent.MaxWalkSpeed` 150.0 _charactermovement)))
    (:`then_2`
      ;[1 1 1] бег
      (if (`self.is sprinting?`)
        (set `CharacterMovementComponent.MaxWalkSpeed` 600.0 _charactermovement)))
    (:`then_3`
      ;[1 1 1] влево вправо норм скорость
      (if (`self.is walk rightleft`)
        (set `CharacterMovementComponent.MaxWalkSpeed` 300.0 (`self.CharacterMovement`))))
    (:`then_4`
      ;[1 1 1] стрейф назад
      (if (== AxisValue -1.0)
        (set `CharacterMovementComponent.MaxWalkSpeed` 150.0 (`self.CharacterMovement`))))))

(event `InputAxis|right`
  (params (AxisValue :type "Float (single-precision)"))
  ;[1 1 1] передвежение
  (`self.AddMovementInput` (`SceneComponent.GetRightVector` (`self.CapsuleComponent`)) AxisValue)
  (set `self.is walk rightleft` (or (== AxisValue 1.0) (== AxisValue -1.0))))

(event `InputAction|equippistol`
  (params (Key :type "Key Structure"))
  ;[1 1 1] пистолет
  (:`Pressed`
    (if (`self.has pistol?`)
      (`/Engine/EditorBlueprintResources/StandardMacros.FlipFlop`
        (:`A`
          (bind _returnvalue (`GameplayStatics.GetActorOfClass` null))
          (bind _output_get (set `self.pistol` _returnvalue))
          (`self.K2_AttachToComponent` _output_get (`self.Mesh`) "socetforpistolequip" "SnapToTarget" "SnapToTarget" "KeepWorld" true)
          (set `self.is pistol euqip` true))
        (:`B`
          (`self.K2_AttachToComponent` (`self.pistol`) (`self.Mesh`) "placeforistol" "SnapToTarget" "SnapToTarget" "KeepWorld" true))))))

(event `InputAction|changecamera`
  (params (Key :type "Key Structure"))
  ;[1 1 1] смена камеры
  (:`Pressed`
    (`/Engine/EditorBlueprintResources/StandardMacros.FlipFlop`
      (:`A`
        (`ActorComponent.Deactivate` (`self.maincamera`))
        (`ActorComponent.Activate` (`self.extracamera`) false)
        (set `self.bUseControllerRotationYaw` true))
      (:`B`
        (`ActorComponent.Deactivate` (`self.extracamera`))
        (`ActorComponent.Activate` (`self.maincamera`) false)
        (set `self.bUseControllerRotationYaw` false)))))

(event `InputAxis|LookupDown`
  (params (AxisValue :type "Float (single-precision)"))
  ;[1 1 1] мышка
  (`self.AddControllerPitchInput` AxisValue))

(event `InputAction|attack`
  (params (Key :type "Key Structure"))
  (:`Pressed`
    (if (and (`self.has pistol?`) (`self.is pistol euqip`))
      (switch `int` (`self.attackanimnomber`)
        (:`Default`
          (`|PlayMontage` (`self.Mesh`)))))))

(event `InputAxis|LockleftDown`
  (params (AxisValue :type "Float (single-precision)"))
  ;[1 1 1] мышка
  (`self.AddControllerYawInput` AxisValue))

(fn `interact`)

(fn `UserConstructionScript`)